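; Sample client component that shows how a mod requests a server-side item spawn from a mod controller, here a standing sign.
; BeginPlay binds to the first MDC_Example controller's actor-spawned event, whose handler is an empty stub with unconnected placeable owner-reset logic.
; The first Tick with a delta of at least one second finds the target controller by name and calls SpawnItem with a template ID and fixed transform.
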(event `Event Actor Spawned`
  (params (actor :type "Actor Object Reference"))
  ;[0 0 0] Sample Client Implementation that spawns a standing sign at 0 0 on Editor Map
)

(event `self.ReceiveBeginPlay`
  ;[0 0 0] Sample Client Implementation that spawns a standing sign at 0 0 on Editor Map
  (if (`KismetSystemLibrary.IsServer`)
    (bind _outactors (`GameplayStatics.GetAllActorsOfClass` "/Game/Mods/Mod2ModRefImpl/MDC_Example.MDC_Example_C"))
    (bind _output_get (set `self.myModController` (`KismetArrayLibrary.Array_Get` _outactors)))
    (add `/Game/Mods/Mod2ModRefImpl/MDC_Example.OnActorSpawned` _output_get (delegate `Event Actor Spawned`))))

(event `self.ReceiveTick`
  (params (DeltaSeconds :type "Float (single-precision)"))
  ;[0 0 0] Sample Client Implementation that spawns a standing sign at 0 0 on Editor Map
  (if (< DeltaSeconds 1.0)
    _
    (elif (not (`self.spawned`))
      (set `self.spawned` true)
      (if (`KismetSystemLibrary.IsServer`)
        (`/Game/Mods/Mod2ModRefImpl/BPL_M2M.ModPrintSimple` "BeginPlay" (`self.DL`))
        (bind _targetmodcontroller (`/Game/Mods/Mod2ModRefImpl/BPL_M2M.findTargetModController` "MDC_Example"))
        (`/Engine/EditorBlueprintResources/StandardMacros.IsValid` _targetmodcontroller
          (:`Is Valid`
            (message `/Game/Systems/Interfaces/BasePlayerCharInterface.GetUniqueID` (`GameplayStatics.GetPlayerCharacter` 0))
            (`/Game/Mods/Mod2ModRefImpl/BPL_M2M.ModPrintSimple` "Invoke Spawn" (`self.DL`))
            (`/Game/Mods/Mod2ModRefImpl/BPL_M2M.SpawnItem` "MDC_Example" _targetmodcontroller 671299999 (`KismetMathLibrary.MakeTransform` (+ (0.0 0.0 355.0) (0.0 0.0 -128.0)) (struct)) "")))))))